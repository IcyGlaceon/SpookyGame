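; BP_Scroll is a collectible scroll actor that the player picks up through interaction.
; Its On Interact override casts the player character to BP_Wizard_Fire, increments that character's Collected count, then runs the parent's interaction.
; If the cast fails, neither the count nor the parent interaction runs.
; Overlap handling is passed straight to the parent class.
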(event EventBeginPlay
  (|CallParentFunction) ; This node is disabled and will not be called.\nDrag off pins to build functionality.
)

(event Collision|EventActorBeginOverlap
  (params (OtherActor :type Actor%20Object%20Reference))
  (|CallParentFunction OtherActor))

(event EventTick
  (params (DeltaSeconds :type Float%20%28single-precision%29))
  (|CallParentFunction DeltaSeconds) ; This node is disabled and will not be called.\nDrag off pins to build functionality.
)

(fn ConstructionScript
  (|CallParentFunction))

(fn OnInteract
  (bind _asbp_wizard_fire (Utilities|Casting|CastToBP_Wizard_Fire (Game|GetPlayerCharacter 0)))
  (Math|Integer|IncrementInt (Variables|/Game/FirstPerson/Blueprints/BP_Wizard_Fire.BP_Wizard_Fire_C|GetCollected _asbp_wizard_fire)
    (:%20%20
      (|CallParentFunction))))
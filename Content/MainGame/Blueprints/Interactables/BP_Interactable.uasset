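; BP_Interactable is an interactable actor that can be triggered while another actor overlaps it.
; Overlap begin and end, filtered by a cast, set CurrentObject to its ObjectName or back to "None".
; The IA_Interact input action calls OnInteract unless CurrentObject is "None".
; OnInteract prints a "Touch" message and destroys the actor.
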(event Input|EnhancedActionEvents|EnhancedInputActionIA_Interact
  (params (ActionValue :type Boolean) (ElapsedSeconds :type Float%20%28double-precision%29) (TriggeredSeconds :type Float%20%28double-precision%29) (InputAction :type Input%20Action%20Object%20Reference :default "/Game/FirstPerson/Input/Actions/IA_Interact.IA_Interact"))
  (:Triggered
    (if (Utilities|Enum|NotEqual(Enum) (Variables|Default|GetCurrentObject) "None")
      (CallFunction|OnInteract))))

(event EventBeginPlay)

(event Collision|EventActorBeginOverlap
  (params (OtherActor :type Actor%20Object%20Reference))
  (Utilities|Casting|CastTo OtherActor)
  (Variables|Default|SetCurrentObject (Variables|Default|GetObjectName)))

(event Collision|EventActorEndOverlap
  (params (OtherActor :type Actor%20Object%20Reference))
  (Utilities|Casting|CastTo OtherActor)
  (Variables|Default|SetCurrentObject "None"))

(fn ConstructionScript)

(fn OnInteract
  (Development|PrintString "Touch")
  (Actor|DestroyActor))
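; BP_Orb is an interactable that, when used, marks one random BP_Scroll in the level.
; OnInteract gathers all scrolls, prints their count, copies the array to every BP_Orb, then calls MarkScroll before the parent interact logic.
; MarkScroll hides the Cylinder component on every scroll, then shows it on a randomly picked one.
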(event Custom|MarkScroll
  (params (Scrolls :type Array%20of%20BP%20Scroll%20Object%20References))
  (if (> (Utilities|Array|Length Scrolls) 0)
    (Utilities|FlowControl|Sequence
      (:then_0
        (for _array_element Scrolls
          (Rendering|SetVisibility (Variables|/Game/MainGame/Blueprints/Interactables/BP_Scroll.BP_Scroll_C|GetCylinder _array_element) false false)))
      (:then_1
        (Rendering|SetVisibility (Variables|/Game/MainGame/Blueprints/Interactables/BP_Scroll.BP_Scroll_C|GetCylinder (.OutItem (Utilities|Array|Random Scrolls))) true false)))))

(event EventBeginPlay
  (|CallParentFunction))

(fn ConstructionScript
  (|CallParentFunction))

(fn OnInteract
  (Utilities|FlowControl|Sequence
    (:then_0
      (bind _outactors (Actor|GetAllActorsOfClass "/Game/MainGame/Blueprints/Interactables/BP_Scroll.BP_Scroll_C"))
      (bind _output_get (Variables|Default|SetScrolls _outactors))
      (Development|PrintString (Utilities|String|ToString(Integer) (Utilities|Array|Length _output_get))))
    (:then_1
      (bind _outactors_2 (Actor|GetAllActorsOfClass "BP_Orb_C"))
      (for _array_element _outactors_2
        (Variables|BP_Orb_C|SetScrolls _array_element (Variables|Default|GetScrolls))))
    (:then_2
      (CallFunction|MarkScroll (Variables|Default|GetScrolls))
      (|CallParentFunction))))
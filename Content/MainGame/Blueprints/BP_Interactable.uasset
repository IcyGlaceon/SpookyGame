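; Base interactable actor that the fire wizard character can use while standing inside its overlap area.
; Overlap with BP_Wizard_Fire stores and prints the object's name as CurrentObject, and leaving resets it to "None".
; The actor handles IA_Interact itself, calling OnInteract when CurrentObject is set.
; OnInteract prints a debug message and destroys the actor.
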(event Input|EnhancedActionEvents|EnhancedInputActionIA_Interact
  (params (ActionValue :type Boolean) (ElapsedSeconds :type Float%20%28double-precision%29) (TriggeredSeconds :type Float%20%28double-precision%29) (InputAction :type Input%20Action%20Object%20Reference :default "/Game/FirstPerson/Input/Actions/IA_Interact.IA_Interact"))
  (:Triggered
    (if (Utilities|Enum|NotEqual(Enum) (Variables|Default|GetCurrentObject) "None")
      (CallFunction|OnInteract))))

(event EventBeginPlay)

(event Collision|EventActorBeginOverlap
  (params (OtherActor :type Actor%20Object%20Reference))
  (bind _objectname (Variables|Default|GetObjectName))
  (Utilities|Casting|CastToBP_Wizard_Fire OtherActor)
  (Variables|Default|SetCurrentObject _objectname)
  (Development|PrintString _objectname))

(event Collision|EventActorEndOverlap
  (params (OtherActor :type Actor%20Object%20Reference))
  (Utilities|Casting|CastToBP_Wizard_Fire OtherActor)
  (Variables|Default|SetCurrentObject "None"))

(fn ConstructionScript)

(fn OnInteract
  (Development|PrintString "Touch")
  (Actor|DestroyActor))